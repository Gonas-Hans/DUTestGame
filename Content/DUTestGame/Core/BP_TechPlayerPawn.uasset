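; Player pawn that gives its player a random set of starting technologies.
; On BeginPlay it caches the BP_TechPlayerState, then InitStartTech picks three distinct random indices from the tech stage array using AddUnique.
; Each picked tech gains one open stage through AddStageByTechIndex on the player state.
; It then prints every tech stage value as debug output.
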(event EventBeginPlay
  (bind _asbp_tech_player_state (Utilities|Casting|CastToBP_TechPlayerState (Variables|GetPlayerState)))
  (Variables|Default|SetTechPlayerStateRef _asbp_tech_player_state)
  (CallFunction|InitStartTech)
  (for _array_element (Default|GetAllTechStages (Variables|Default|GetTechPlayerStateRef))
    (Development|PrintString (Utilities|String|ToString(Integer) _array_element))))

(event Collision|EventActorBeginOverlap
  (params (OtherActor :type Actor%20Object%20Reference)))

(event EventTick
  (params (DeltaSeconds :type Float%20%28single-precision%29)))

(fn ConstructionScript)

(fn InitStartTech
  ;[0.941 0.5144 1] Выбираем три случайные технологии т.е. три случайных индекса в массиве технологических очков ( 0 индекс - первая технология, 1- вторая и т.д.)
  (while (< (Utilities|Array|Length (LocalVariables|GetIndexesOpenTech)) 3)
    (Utilities|Array|AddUnique (LocalVariables|GetIndexesOpenTech) (.OutIndex (Utilities|Array|Random (Default|GetAllTechStages (Variables|Default|GetTechPlayerStateRef))))))
  ;[0.6512 1 0.4623] Добавляем по одной открытой стадии технологиям по выбранным ранее индексам
  (for _array_element (LocalVariables|GetIndexesOpenTech)
    (Default|AddStagebyTechIndex (Variables|Default|GetTechPlayerStateRef) _array_element 1)))