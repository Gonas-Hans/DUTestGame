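; BP_TechPlayerState is a player state that holds a player's point balance and per-tech point totals.
; Getter and add functions read or increase the balance and the TechPoints array entries, addressed by tech index.
; SubtractPlayerPoints deducts only when the balance covers the cost, but its returned comparison uses the updated balance, so a successful deduction can report false.
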(event EventBeginPlay)

(event EventTick
  (params (DeltaSeconds :type Float%20%28single-precision%29)))

(fn ConstructionScript)

(fn GetPlayerPoints
  (return (Variables|Default|GetPlayerPoints)))

(fn AddPlayerPoints
  (params (Points :type Integer))
  (Variables|Default|SetPlayerPoints (+ Points (Variables|Default|GetPlayerPoints))))

(fn GetTechPoints
  (params (TechIndex :type Integer))
  (return (Utilities|Array|Get(acopy) (Variables|Default|GetTechPoints) TechIndex)))

(fn AddTechPoints
  (params (TechIndex :type Integer) (Points :type Integer))
  (Utilities|Array|SetArrayElem (Variables|Default|GetTechPoints) TechIndex (+ Points (Utilities|Array|Get(acopy) (Variables|Default|GetTechPoints) TechIndex))))

(fn SubtractPlayerPoints
  (params (Points :type Integer))
  (if (<= Points (Variables|Default|GetPlayerPoints))
    (Variables|Default|SetPlayerPoints (- (Variables|Default|GetPlayerPoints) Points)))
  (return (<= Points (Variables|Default|GetPlayerPoints))))